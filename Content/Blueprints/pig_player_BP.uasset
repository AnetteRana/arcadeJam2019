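; Player pig that the user moves and dashes, eating food to gain happiness, weight and hunger points.
; Tick applies axis movement with smoothed rotation, drains hunger and prints a message for starvation or reaching the weight goal.
; Food overlaps update stats and, through a Widget_BP found at BeginPlay, log the meal, destroy the food and play audio.
; Dashing costs hunger; its cooldown delay and football logic are disconnected.
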(event `self.ReceiveActorBeginOverlap`
  (params (OtherActor :type "Actor Object Reference"))
  (bind _mywidget (`self.myWidget`))
  ;[1 1 1] overlap food
  (bind _asfood (cast `/Game/Blueprints/food` OtherActor))
  (`|ExecutionSequence`
    (:`then_0`
      (set `self.happiness` (+ (`self.happiness`) (`/Game/Blueprints/food.happinessPoints` _asfood))))
    (:`then_1`
      (bind _output_get (set `self.weight` (+ (`/Game/Blueprints/food.weightGained` _asfood) (stale _output_get)))))
    (:`then_2`
      (bind _output_get_2 (set `self.hunger` (+ (stale _output_get_2) (`/Game/Blueprints/food.hungerRemoved` _asfood))))
      (if (> _output_get_2 100.0)
        (set `self.hunger` 100.0)))
    (:`then_3`
      (if (`KismetSystemLibrary.IsValid` (`self.myWidget`))
        (set `/Game/Blueprints/widget_BP.happiness` (`self.happiness`) _mywidget)
        (set `/Game/Blueprints/widget_BP.weight` (`self.weight`) _mywidget)
        (set `/Game/Blueprints/widget_BP.hunger` (`self.hunger`) _mywidget)
        (`/Game/Blueprints/widget_BP.log action` _mywidget (`KismetTextLibrary.Conv_StringToText` (`KismetStringLibrary.Concat_StrStr` "Ate " (`/Game/Blueprints/food.foodName` _asfood))))
        (`self.K2_DestroyActor` OtherActor)
        (`AudioComponent.Play` (`self.Audio`) 0.0)))))

(event `self.ReceiveBeginPlay`
  ;[1 1 1] BeginPlay
  ;[1 1 1] Get GUI
  (bind _foundwidgets (`WidgetBlueprintLibrary.GetAllWidgetsOfClass` "/Game/Blueprints/widget_BP.widget_BP_C"))
  (set `self.myWidget` (`|GetArrayItem` _foundwidgets))
  ;[1 1 1] if no GUI... try again
  (if (not (`KismetSystemLibrary.IsValid` (`self.myWidget`)))
    (`KismetSystemLibrary.Delay` 0.2)
    (bind _foundwidgets_2 (`WidgetBlueprintLibrary.GetAllWidgetsOfClass` "/Game/Blueprints/widget_BP.widget_BP_C"))
    (set `self.myWidget` (`|GetArrayItem` _foundwidgets_2))))

(event `Key|Escape`
  (params (Key :type "Key Structure"))
  ;[1 1 1] exit game
  (:`Pressed`
    (`KismetSystemLibrary.QuitGame` null "Quit")))

(event `self.ReceiveTick`
  (params (DeltaSeconds :type "Float (single-precision)"))
  (bind _returnvalue (`KismetMathLibrary.MakeVector` (`self.GetInputAxisValue`) (`self.GetInputAxisValue`)))
  (`|ExecutionSequence`
    (:`then_0`
      ;[1 1 1] movement
      (`self.AddMovementInput` _returnvalue (`self.moveSpeed`))
      ;;[1 1 1] if moving = rotate too
      (if (or (!= (`self.GetInputAxisValue`) 0.0) (!= (`self.GetInputAxisValue`) 0.0))
        (`self.K2_SetActorRelativeRotation` (`KismetMathLibrary.RLerp` (`KismetMathLibrary.Conv_VectorToRotator` _returnvalue) (`self.K2_GetActorRotation`) 0.5 true))))
    (:`then_1`
      (if (<= (`self.hunger`) 0.0)
        (`KismetSystemLibrary.PrintString` "STARVED TO DEATH")
        (elif (>= (`self.weight`) 100.0)
          (`KismetSystemLibrary.PrintString` "GOOD GAME OVER"))))
    (:`then_2`
      ;[1 1 1] updateWidget
      (bind _output_get (set `self.hunger` (- (stale _output_get) (* DeltaSeconds 5.0))))
      (if (`KismetSystemLibrary.IsValid` (`self.myWidget`))
        (set `/Game/Blueprints/widget_BP.hunger` (`self.hunger`) (`self.myWidget`))))))

(event `InputAction|ButtonA`
  (params (Key :type "Key Structure"))
  ;[1 1 1] button A - Dash!
  (:`Pressed`
    (if (`self.sprintIsReady`)
      (set `self.sprintIsReady` false)
      (set `MovementComponent.Velocity` (* (`KismetMathLibrary.GetForwardVector` (`self.K2_GetActorRotation`)) 3000.0) (`self.MovementComponent`))
      (bind _output_get (set `self.hunger` (- (stale _output_get) 5.0)))
      (set `self.sprintIsReady` true))))

(fn `UserConstructionScript`)