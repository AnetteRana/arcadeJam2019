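; Pig game mode that scatters random pickups and props (fruit, puddles, footballs) across the level at BeginPlay.
; SpawnLevelStuff walks a 9x9 grid around the origin, skips the center cell, and spawns one random class per cell with random XY jitter.
; ClearLevelStuffThenSpawnNew destroys every actor tagged "spawnable" and then runs the spawn pass again for a fresh layout.
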(event `self.ReceiveBeginPlay`
  (`self.SpawnLevelStuff`))

(fn `ClearLevelStuff_thenSpawnNew`
  (bind _outactors (`GameplayStatics.GetAllActorsWithTag` "spawnable"))
  (for _array_element _outactors
    (`self.K2_DestroyActor` _array_element))
  (`self.SpawnLevelStuff`))

(fn `SpawnLevelStuff`
  ;[1 1 1] outer loop
  (for _index (range 9)
    (for _index_2 (range 9)
      (bind _returnvalue (`KismetMathLibrary.Conv_IntToDouble` (- 2000 (* _index_2 500))))
      (bind _returnvalue_2 (`KismetMathLibrary.Conv_IntToDouble` (- 2000 (* _index 500))))
      (if (or (!= _returnvalue 0.0) (!= _returnvalue_2 0.0))
        (`|ExecutionSequence`
          (:`then_0`
            (switch `int` (`KismetMathLibrary.RandomInteger` 7)
              (:`0`
                (set `self.nextActorToSpawn` "/Game/Blueprints/puddle.puddle_C"))
              (:`1`
                (set `self.nextActorToSpawn` "/Game/Blueprints/fotball.fotball_C"))
              (:`2`
                (set `self.nextActorToSpawn` "/Game/Blueprints/foods/apple.apple_C"))
              (:`3`
                (set `self.nextActorToSpawn` "/Game/Blueprints/foods/pear.pear_C"))
              (:`4`
                (set `self.nextActorToSpawn` "/Game/Blueprints/foods/strawberry.strawberry_C"))
              (:`5`
                (set `self.nextActorToSpawn` "/Game/Blueprints/foods/banana.banana_C"))
              (:`6`
                (set `self.nextActorToSpawn` "/Game/Blueprints/foods/apple.apple_C"))
              (:`7`
                (set `self.nextActorToSpawn` "/Game/Blueprints/foods/pear.pear_C"))))
          (:`then_1`
            (`|SpawnActorFromClass` (`self.nextActorToSpawn`) (`KismetMathLibrary.MakeTransform` (`KismetMathLibrary.MakeVector` (+ _returnvalue (`KismetMathLibrary.RandomFloatInRange` -200.0 200.0)) (+ _returnvalue_2 (`KismetMathLibrary.RandomFloatInRange` -200.0 200.0)) 0.0)) "Undefined" "OverrideRootScale" null null)))))))

(fn `UserConstructionScript`)