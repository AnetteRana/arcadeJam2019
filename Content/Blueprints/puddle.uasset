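; Puddle actor that raises the pig player's happiness while the player is nearby.
; Each Tick measures the distance from the player pawn to the Sphere component and, within a fixed radius, calls UpdateHappiness on pig_player_BP with AmountHappiness.
; A timestamp cooldown limits the reward to once every couple of seconds.
; A disconnected branch that accumulates PlayerBallInteractionTime never runs.
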(event `self.ReceiveTick`
  (params (DeltaSeconds :type "Float (single-precision)"))
  (bind _returnvalue (`GameplayStatics.GetTimeSeconds`))
  (if (< (`KismetMathLibrary.VSize` (- (`self.K2_GetActorLocation` (`GameplayStatics.GetPlayerPawn` 0)) (`SceneComponent.K2_GetComponentLocation` (`self.Sphere`)))) 200.0)
    (if (>= _returnvalue (+ (`self.lastBallHappyTime`) 2.0))
      (set `self.lastBallHappyTime` _returnvalue)
      (bind _aspig_player_bp (cast `/Game/Blueprints/pig_player_BP` (`GameplayStatics.GetPlayerPawn` 0)))
      (`/Game/Blueprints/pig_player_BP.updateHappiness` _aspig_player_bp (`self.amountHappiness`)))))

(fn `UserConstructionScript`)