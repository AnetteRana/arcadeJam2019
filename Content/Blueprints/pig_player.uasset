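; Player-controlled pig that eats food to change its Happiness, Weight and Hunger, with Hunger draining steadily each Tick.
; Food overlaps add stats with Hunger capped, then, if the HUD widget is valid, update it, log the meal, destroy the food and play audio.
; BeginPlay finds that widget with one delayed retry, and Tick applies axis movement with lerped facing.
; Football overlaps only print ball speed, and Escape quits.
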(event `self.ReceiveActorBeginOverlap`
  (params (OtherActor :type "Actor Object Reference"))
  (bind _mywidget (`self.myWidget`))
  ;[1 1 1] overlap food
  (bind _asfood (cast `/Game/Blueprints/food` OtherActor)
    (:`then`
      (`|ExecutionSequence`
        (:`then_0`
          (set `self.happiness` (+ (`self.happiness`) (`/Game/Blueprints/food.happinessPoints` _asfood))))
        (:`then_1`
          (bind _output_get (set `self.weight` (+ (`/Game/Blueprints/food.weightGained` _asfood) (stale _output_get)))))
        (:`then_2`
          (bind _output_get_2 (set `self.hunger` (+ (stale _output_get_2) (`/Game/Blueprints/food.hungerRemoved` _asfood))))
          (if (> _output_get_2 100.0)
            (set `self.hunger` 100.0)))
        (:`then_3`
          (if (`KismetSystemLibrary.IsValid` (`self.myWidget`))
            (set `/Game/Blueprints/widget_BP.happiness` (`self.happiness`) _mywidget)
            (set `/Game/Blueprints/widget_BP.weight` (`self.weight`) _mywidget)
            (set `/Game/Blueprints/widget_BP.hunger` (`self.hunger`) _mywidget)
            (`/Game/Blueprints/widget_BP.log action` _mywidget (`KismetTextLibrary.Conv_StringToText` (`KismetStringLibrary.Concat_StrStr` "Ate " (`/Game/Blueprints/food.foodName` _asfood))))
            (`self.K2_DestroyActor` OtherActor)
            (`AudioComponent.Play` (`self.Audio`) 0.0)))))
    (:`CastFailed`
      ;[1 1 1] overlap fotball
      (bind _asfotball (cast `/Game/Blueprints/fotball` OtherActor))
      (bind _returnvalue (`KismetMathLibrary.VSize` (`self.GetVelocity` _asfotball)))
      (if (> _returnvalue 0.0)
        _
        (else
          _))
      (`KismetSystemLibrary.PrintString` (`KismetStringLibrary.Conv_DoubleToString` _returnvalue)))))

(event `self.ReceiveBeginPlay`
  ;[1 1 1] BeginPlay
  ;[1 1 1] Get GUI
  (bind _foundwidgets (`WidgetBlueprintLibrary.GetAllWidgetsOfClass` "/Game/Blueprints/widget_BP.widget_BP_C"))
  (set `self.myWidget` (`|GetArrayItem` _foundwidgets))
  ;[1 1 1] if no GUI... try again
  (if (not (`KismetSystemLibrary.IsValid` (`self.myWidget`)))
    (`KismetSystemLibrary.Delay` 0.2)
    (bind _foundwidgets_2 (`WidgetBlueprintLibrary.GetAllWidgetsOfClass` "/Game/Blueprints/widget_BP.widget_BP_C"))
    (set `self.myWidget` (`|GetArrayItem` _foundwidgets_2))))

(event `Key|Escape`
  (params (Key :type "Key Structure"))
  ;[1 1 1] exit game
  (:`Pressed`
    (`KismetSystemLibrary.QuitGame` null "Quit")))

(event `self.ReceiveTick`
  (params (DeltaSeconds :type "Float (single-precision)"))
  (bind _returnvalue (`KismetMathLibrary.MakeVector` (`self.GetInputAxisValue`) (`self.GetInputAxisValue`)))
  (`|ExecutionSequence`
    (:`then_0`
      (bind _output_get (set `self.hunger` (- (stale _output_get) (* DeltaSeconds 5.0))))
      ;[1 1 1] updateWidget
      (if (`KismetSystemLibrary.IsValid` (`self.myWidget`))
        (set `/Game/Blueprints/widget_BP.hunger` (`self.hunger`) (`self.myWidget`))))
    (:`then_1`
      ;[1 1 1] movement
      (`self.AddMovementInput` _returnvalue (`self.moveSpeed`))
      (`self.K2_SetActorRelativeRotation` (`KismetMathLibrary.RLerp` (`KismetMathLibrary.Conv_VectorToRotator` _returnvalue) (`self.K2_GetActorRotation`) 0.5 true)))))

(fn `UserConstructionScript`)