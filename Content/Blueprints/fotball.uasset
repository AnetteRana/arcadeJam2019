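; A football the pig player can push around to gain happiness.
; Any actor overlap applies a velocity-change impulse to the Sphere along the player pawn's forward vector.
; While the ball moves near the player, Tick accumulates interaction time and raises the pig's happiness through UpdateHappiness, throttled by a short cooldown.
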(event `self.ReceiveActorBeginOverlap`
  (params (OtherActor :type "Actor Object Reference"))
  ;[1 1 1] movement
  (`PrimitiveComponent.AddImpulse` (`self.Sphere`) (* (`self.GetActorForwardVector` (`GameplayStatics.GetPlayerPawn` 0)) 400.0) "None" true))

(event `self.ReceiveTick`
  (params (DeltaSeconds :type "Float (single-precision)"))
  (bind _returnvalue (`GameplayStatics.GetTimeSeconds`))
  (if (and (< (`KismetMathLibrary.VSize` (- (`self.K2_GetActorLocation` (`GameplayStatics.GetPlayerPawn` 0)) (`SceneComponent.K2_GetComponentLocation` (`self.Sphere`)))) 300.0) (> (`KismetMathLibrary.VSize` (`SceneComponent.GetComponentVelocity` (`self.Sphere`))) 15.0))
    (bind _output_get (set `self.playerBallInteractionTime` (+ DeltaSeconds (stale _output_get))))
    (if (>= _returnvalue (+ (`self.lastBallHappyTime`) 2.0))
      (set `self.lastBallHappyTime` _returnvalue)
      (bind _aspig_player_bp (cast `/Game/Blueprints/pig_player_BP` (`GameplayStatics.GetPlayerPawn` 0)))
      (`/Game/Blueprints/pig_player_BP.updateHappiness` _aspig_player_bp 10))))

(fn `UserConstructionScript`)